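; BP_Synchronization is a small debug Blueprint that appears to test value synchronization between a dedicated server and clients.
; On BeginPlay, only a dedicated server sets NewVar0 and passes it to the Printint custom event, which prints it on screen.
; Disconnected leftover logic would increment the variable on the server after a delay or print it on non-server instances, but it never runs.
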(event Custom|Print%20int
  (params (NewVar_0 :type Integer))
  (Development|PrintString (Utilities|String|ToString(Integer) NewVar_0) true true "(R=0.000000,G=0.660000,B=1.000000,A=1.000000)" 12.0))

(event EventTick
  (params (DeltaSeconds :type Float%20%28single-precision%29)))

(event EventBeginPlay
  (if (Networking|IsDedicatedServer)
    (Variables|Default|SetNewVar_0 22)
    (CallFunction|PrintInt (Variables|Default|GetNewVar_0))))

(fn ConstructionScript)